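; Base 2D action character with faction-based melee combat, health, stun and defeat.
; Its hitbox damages opposing-faction characters on overlap and briefly freezes both through custom time dilation for hit-stop.
; Received hits play a sound, then trigger either defeat or a timed stun via animation node jumps, with timer-driven sprite shake during stun.
; CanAct blocks actions while attacking, stunned or defeated.
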(event OnComponentBeginOverlap(HitBox)
  (params (OverlappedComponent :type Primitive%20Component%20Object%20Reference) (OtherActor :type Actor%20Object%20Reference) (OtherComp :type Primitive%20Component%20Object%20Reference) (OtherBodyIndex :type Integer) (bFromSweep :type Boolean) (SweepResult :type Hit%20Result%20Structure%20%28by%20ref%29))
  (bind _asbp_action_char (Utilities|Casting|CastToBP_ActionChar OtherActor))
  (if (!= (Variables|BP_ActionChar_C|GetFaction _asbp_action_char) (Variables|Default|GetFaction))
    (CallFunction|RecieveAttack _asbp_action_char 25.0)
    (CallFunction|HitStopSequence _asbp_action_char 0.08)
    (CallFunction|HitStopSequence 0.08)))

(event Custom|Hit%20Stop%20Sequence
  (params (Duration :type Float%20%28single-precision%29))
  (Variables|Default|SetCustomTimeDilation 0.0)
  (Utilities|FlowControl|RetriggerableDelay Duration)
  (Variables|Default|SetCustomTimeDilation 1.0))

(event Custom|ShakeSprite
  (bind _sprite_location (Variables|Default|GetSprite%20Location))
  (bind _isa (Utilities|FlowControl|FlipFlop)
    (:A
      _)
    (:B
      _))
  (Transformation|SetRelativeLocation (Variables|Default|GetSprite) (Math|Vector|MakeVector (+ (.x _sprite_location) (Math|Float|SelectFloat (Variables|Default|GetSpriteShakeDistance) (* (Variables|Default|GetSpriteShakeDistance) -1.0) _isa)) (.y _sprite_location) (.z _sprite_location)) false false))

(event EventBeginPlay
  (CallFunction|SetHitboxCollision false)
  (Variables|Default|SetCurrentHealth (Variables|Default|GetMaxHealth))
  (Variables|Default|SetSprite%20Location (Variables|/Script/Engine.SceneComponent|GetRelativeLocation (Variables|Default|GetSprite))))

(event Collision|EventActorBeginOverlap
  (params (OtherActor :type Actor%20Object%20Reference)))

(event EventTick
  (params (DeltaSeconds :type Float%20%28single-precision%29)))

(fn ConstructionScript)

(fn SetHitboxCollision
  (params (Set%20Active :type Boolean))
  (if Set%20Active
    (Collision|SetCollisionEnabled (Variables|Default|GetHitBox) "QueryOnly")
    (else
      (Collision|SetCollisionEnabled (Variables|Default|GetHitBox) "NoCollision"))))

(fn RecieveAttack
  (params (Damage :type Float%20%28double-precision%29))
  (if (not (Variables|Default|GetIsDefeated))
    (Audio|PlaySoundatLocation "/Game/SFX/S_Hit_Cue.S_Hit_Cue" (Transformation|GetActorLocation) "0, 0, 0" 1.0 1.0 0.0 0 0 0 0)
    (Variables|Default|SetCurrentHealth (- (Variables|Default|GetCurrentHealth) Damage))
    (if (<= (Variables|Default|GetCurrentHealth) 0.0)
      (Class|PaperZDAnimInstance|JumptoNode (Class|PaperZDCharacter|GetAnimInstance) "JumpDefeated" "None")
      (Variables|Default|SetIsDefeated true)
      (Collision|SetCollisionEnabled (Variables|Default|GetCapsuleComponent) "NoCollision")
      (else
        (Variables|Default|SetStunned true)
        (Default|CallStunStateChanged true)
        (Class|PaperZDAnimInstance|JumptoNode (Class|PaperZDCharacter|GetAnimInstance) "JumpStunned" "None")
        (Utilities|Time|SetTimerbyEvent (EventDispatchers|CreateEvent :!event ClearStun) (Variables|Default|GetStun%20Length))
        (bind _returnvalue (Utilities|Time|SetTimerbyEvent (EventDispatchers|CreateEvent :!event Custom|ShakeSprite) (Variables|Default|GetSprite%20Shake%20Frequency) true))
        (Variables|Default|SetSprite%20Shake%20Handle _returnvalue)))))

(fn ClearStun
  (Variables|Default|SetStunned false)
  (Default|CallStunStateChanged false)
  (Utilities|Time|ClearandInvalidateTimerbyHandle (Variables|Default|GetSprite%20Shake%20Handle))
  (Transformation|SetRelativeLocation (Variables|Default|GetSprite) (Variables|Default|GetSprite%20Location) false false))

(fn CanAct
  (return (Math|Boolean|ANDBoolean (not (Variables|Default|GetIsAttacking)) (not (Variables|Default|GetIsDefeated)) (not (Variables|Default|GetStunned)))))